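; Road barrier actor that can scatter its mesh slightly for a less uniform placement in the level.
; On BeginPlay, if Randomize is set, it teleports the mesh by random relative X and Y offsets and adds a random yaw, each within configurable min/max ranges.
; The construction script is empty, so the variation appears only at runtime and differs on each play.
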(event `self.ReceiveBeginPlay`
  (bind (_relativelocation_x _relativelocation_y _relativelocation_z) (`KismetMathLibrary.BreakVector` (`SceneComponent.RelativeLocation` (`self.Mesh`))))
  (bind (_relativerotation_roll _relativerotation_pitch _relativerotation_yaw) (`KismetMathLibrary.BreakRotator` (`SceneComponent.RelativeRotation` (`self.Mesh`))))
  ;[1 1 1] Set random location
  (if (`self.Randomize?`)
    (`SceneComponent.K2_SetRelativeLocation` (`self.Mesh`) (`KismetMathLibrary.MakeVector` (+ _relativelocation_x (`KismetMathLibrary.RandomFloatInRange` (`self.RandomMinLocation`) (`self.RandomMaxLocation`))) (+ _relativelocation_y (`KismetMathLibrary.RandomFloatInRange` (`self.RandomMinLocation`) (`self.RandomMaxLocation`))) _relativelocation_z) false true)
    ;[1 1 1] Set Random Rotation
    (`SceneComponent.K2_SetRelativeRotation` (`self.Mesh`) (`KismetMathLibrary.MakeRotator` _relativerotation_roll _relativerotation_pitch (+ _relativerotation_yaw (`KismetMathLibrary.RandomFloatInRange` (`self.RandomMinRotation`) (`self.RandomMaxRotation`)))) false false)))

(fn `UserConstructionScript`)